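; VR game mode that runs a wave-based enemy game from start to game over.
; At BeginPlay it gathers enemy spawners and a menu-like actor by interface, hiding that actor during play and showing it again when waves run out.
; Each wave plays a color timeline into a floor material parameter collection, then shuffles spawners, messages as many as that wave's enemy count, and schedules the next wave by timer.
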(event Custom|GameOver
  (bind _mref (Variables|Default|GetMRef))
  (Rendering|SetActorHiddenInGame _mref false)
  (Collision|SetActorEnableCollision _mref true))

(event Custom|HandleSpawningWave
  (if (> (Variables|Default|GetWaveNumber) (Utilities|Array|LastIndex (Variables|Default|GetEnemiesPeWave)))
    (CallFunction|GameOver)
    (else
      (bind _color (Timeline|Color PlayFromStart)
        (:Update
          (Rendering|Material|SetVectorParameterValue "/Game/Materials/BPC_Floor.BPC_Floor" "RedColor" _color :!class /Script/Engine.KismetMaterialLibrary))
        (:Finished
          (CallFunction|SpawnEnemyWave))))))

(event EventBeginPlay
  (bind _outactors (Actor|GetAllActorswithInterface "/Game/InterFace/BPL_EnemySpwan.BPL_EnemySpwan_C"))
  (Variables|Default|SetEnmySpwans _outactors)
  (bind _outactors_2 (Actor|GetAllActorswithInterface "/Game/InterFace/BPL_M.BPL_M_C"))
  (Variables|Default|SetMRef (Utilities|Array|Get(acopy) _outactors_2)))

(event EventStartGame
  (bind _mref (Variables|Default|GetMRef))
  (Class|BPLPlayer|ResetSore(Message) (Game|Player|GetPlayerPawn 0))
  (Variables|Default|SetWaveNumber 0)
  (Rendering|SetActorHiddenInGame _mref true)
  (Collision|SetActorEnableCollision _mref false)
  (CallFunction|HandleSpawningWave))

(fn ConstructionScript)

(fn SpawnEnemyWave
  (Utilities|Array|Shuffle (Variables|Default|GetEnmySpwans))
  (for _index (range 0 (- (Utilities|Array|Get(acopy) (Variables|Default|GetEnemiesPeWave) (Variables|Default|GetWaveNumber)) 1))
    (Class|BPLEnemySpwan|HandleEnemySpwaner(Message) (Utilities|Array|Get(acopy) (Variables|Default|GetEnmySpwans) _index)))
  (Math|Integer|IncrementInt (Variables|Default|GetWaveNumber)
    (:%20%20
      (Utilities|Time|SetTimerbyFunctionName 0 "HandleSpawningWave" (Variables|Default|GetDelayPreWave)))))